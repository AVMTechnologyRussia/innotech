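; Player pawn for VR and desktop that tracks gaze and "thinking" time and shows a microphone indicator.
; BeginPlay picks floor tracking for a headset, or controller look, a height offset and a screen mic widget otherwise.
; Each tick traces from the camera for PhysicsBody objects; a looping timer accumulates BadLook while nothing is hit.
; A separate pausable timer accumulates Thinking, which is printed every tick for debugging.
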(event `InputAxis|LookRight`
  (params (AxisValue :type "Float (single-precision)"))
  (`self.AddControllerYawInput` AxisValue))

(event `InputAxis|LookUp`
  (params (AxisValue :type "Float (single-precision)"))
  (`self.AddControllerPitchInput` AxisValue))

(event `SetVisibitilyMic`
  (params (NewParam :type Boolean))
  (if (`HeadMountedDisplayFunctionLibrary.IsHeadMountedDisplayEnabled`)
    (`SceneComponent.SetVisibility` (`self.Widget`) NewParam false)
    (else
      (`Widget.SetVisibility` (`/Game/Blueprints/Widgets/VoiceActivate.Image_77` (`self.MicWidgetRef`)) (select `bool` NewParam :`false` "Hidden" :`true` "Visible" :!type "ESlateVisibility Enum")))))

(event `self.ReceiveBeginPlay`
  (bind _returnvalue (`HeadMountedDisplayFunctionLibrary.IsHeadMountedDisplayEnabled`))
  (`self.StartTimeBadLook`)
  (set `CameraComponent.bUsePawnControlRotation` (not _returnvalue) (`self.Camera`))
  (if _returnvalue
    (`HeadMountedDisplayFunctionLibrary.SetTrackingOrigin` "Floor")
    (else
      (`SceneComponent.K2_AddLocalOffset` (`self.VRRoot`) (`KismetMathLibrary.MakeVector` 0.0 0.0 (`self.DefaultPlayerHeight`)) false false)
      (bind _returnvalue_2 (`|CreateWidget` "/Game/Blueprints/Widgets/VoiceActivate.VoiceActivate_C"))
      (bind _output_get (set `self.MicWidgetRef` _returnvalue_2))
      (`UserWidget.AddToViewport` _output_get 0))))

(event `StartTimeBadLook`
  (bind _returnvalue (`KismetSystemLibrary.K2_SetTimerDelegate` (delegate `TimeBadLook`) 0.1 true))
  (set `self.TimerBadLook` _returnvalue))

(event `TimeBadLook`
  (if (`self.Bool`)
    (set `self.BadLook` (+ 0.1 (`self.BadLook`)))))

(event `self.ReceiveTick`
  (params (DeltaSeconds :type "Float (single-precision)"))
  (`|ExecutionSequence`
    (:`then_0`
      (bind _newparam (`self.LineTrace`))
      (if _newparam
        (set `self.Bool` false)
        (else
          (set `self.Bool` true))))
    (:`then_1`
      (`KismetSystemLibrary.PrintString` (`KismetStringLibrary.Conv_DoubleToString` (`self.Thinking`)) true true (struct :`G` 0.66 :`B` 1.0 :`A` 1.0) 0.0))))

(event `StartTimeThinking`
  (bind _returnvalue (`KismetSystemLibrary.K2_SetTimerDelegate` (delegate `TimeThinking`) 0.1 true))
  (set `self.TimerThinking` _returnvalue))

(event `TimeThinking`
  (set `self.Thinking` (+ 0.1 (`self.Thinking`))))

(event `PauseTimerThinking`
  (`KismetSystemLibrary.K2_PauseTimerHandle` (`self.TimerThinking`)))

(event `UnpauseTimerThinking`
  (`KismetSystemLibrary.K2_UnPauseTimerHandle` (`self.TimerThinking`)))

(fn `LineTrace`
  (returns (NewParam :type Boolean))
  (bind _camera (`self.Camera`))
  (bind _returnvalue (`SceneComponent.K2_GetComponentLocation` _camera))
  (bind (_outhit _returnvalue_2) (`KismetSystemLibrary.LineTraceSingleForObjects` _returnvalue (+ _returnvalue (* (`SceneComponent.GetForwardVector` _camera) 1000.0)) (`|MakeArray` "ObjectTypeQuery4" :!type "EObjectTypeQuery Enum")))
  (return _returnvalue_2))

(fn `UserConstructionScript`)